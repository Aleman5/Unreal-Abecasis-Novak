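; SKM_Door_main is an interactive skeletal mesh door that the player opens and closes with the E key.
; A Box overlap enables the actor's input for the first player controller, and leaving the box disables it.
; Each press flips the OpernClose flag and plays the door montage on the SkeletalMesh, forward to open and at negative play rate to close.
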(event `self.Box.OnComponentBeginOverlap`
  (params (OverlappedComponent :type "PrimitiveComponent Object Reference") (OtherActor :type "Actor Object Reference") (OtherComp :type "PrimitiveComponent Object Reference") (OtherBodyIndex :type Integer) (bFromSweep :type Boolean) (SweepResult :type "HitResult Structure (by ref)"))
  ;[1 1 1] Basic Setting
  (`self.EnableInput` (`GameplayStatics.GetPlayerController` 0)))

(event `self.Box.OnComponentEndOverlap`
  (params (OverlappedComponent :type "PrimitiveComponent Object Reference") (OtherActor :type "Actor Object Reference") (OtherComp :type "PrimitiveComponent Object Reference") (OtherBodyIndex :type Integer))
  ;[1 1 1] Basic Setting
  (`self.DisableInput` (`GameplayStatics.GetPlayerController` 0)))

(event `Key|E`
  (params (Key :type "Key Structure"))
  ;[1 1 1] Open & Close Door
  (:`Pressed`
    (if (`self.OpernClose`)
      (set `self.OpernClose` false)
      (`|PlayMontage` (`self.SkeletalMesh`) "/Game/HQ_ResidentialHouse/Meshes/DoorMain/AnimMainDoor_Montage.AnimMainDoor_Montage" -1.0)
      (else
        (set `self.OpernClose` true)
        (`|PlayMontage` (`self.SkeletalMesh`) "/Game/HQ_ResidentialHouse/Meshes/DoorMain/AnimMainDoor_Montage.AnimMainDoor_Montage")))))

(fn `UserConstructionScript`)